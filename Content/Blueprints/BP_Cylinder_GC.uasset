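; BP_Cylinder_GC is a destructible Chaos Geometry Collection cylinder that drops a random projectile pickup when broken.
; With DestroyOnSpawn set, it spawns a short-lived FS_MasterField_Temp at its location on BeginPlay to apply a radial field.
; The first break event spawns one of four pickup sizes and optionally plays audio, while component hits wake the rigid body.
; Tick destroys the actor once that pickup is no longer valid.
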(event OnChaosBreakEvent(GeometryCollectionComponent)
  (params (BreakEvent :type Chaos%20Break%20Event%20Structure%20%28by%20ref%29))
  (if (not (Variables|Default|GetSpawnedPickUp))
    (CallFunction|SpawnPickUp)
    (Variables|Default|SetSpawnedPickUp true)
    (if (Variables|Default|GetPlayAudio)
      (bind _returnvalue (AddComponent|AddAudioComponent false))
      (bind _output_get (Variables|Default|SetAudio _returnvalue))
      (Audio|Components|Audio|SetVolumeMultiplier _returnvalue 0.7 :!class /Script/Engine.AudioComponent)
      (Audio|Components|Audio|Play _returnvalue 0.0))))

(event OnComponentHit(GeometryCollectionComponent)
  (params (HitComponent :type Primitive%20Component%20Object%20Reference) (OtherActor :type Actor%20Object%20Reference) (OtherComp :type Primitive%20Component%20Object%20Reference) (NormalImpulse :type Vector :default "0, 0, 0") (Hit :type Hit%20Result%20Structure%20%28by%20ref%29))
  (Class|PrimitiveComponent|WakeRigidBody (Variables|Default|GetGeometryCollectionComponent) "None"))

(event EventBeginPlay
  (bind _fieldscale (Variables|Default|GetFieldScale))
  (Variables|Default|SetSpawnedPickUp false)
  (if (Variables|Default|GetDestroyOnSpawn)
    (bind _returnvalue (Game|SpawnActorfromClass "/Game/Chaos/FS_MasterField_Temp.FS_MasterField_Temp_C" (Math|Transform|MakeTransform (.location (Transformation|GetActorTransform)) "0, 0, 0" (Math|Vector|MakeVector _fieldscale _fieldscale _fieldscale)) "Undefined" "MultiplyWithRoot" 0 0))
    (Variables|/Game/Chaos/FS_MasterField_Temp.FS_MasterField_Temp_C|SetRadial%20Magnitude _returnvalue (Variables|Default|GetRadialMagnitude))
    (Actor|SetLifeSpan _returnvalue 0.1)
    (Default|CETrigger _returnvalue)
    (Variables|Default|SetDestroyed true)))

(event Collision|EventActorBeginOverlap
  (params (OtherActor :type Actor%20Object%20Reference)))

(event EventTick
  (params (DeltaSeconds :type Float%20%28single-precision%29))
  (if (and (Variables|Default|GetSpawnedPickUp) (not (Utilities|IsValid (Variables|Default|GetPickUpActor))))
    (Actor|DestroyActor)))

(fn ConstructionScript)

(fn SpawnPickUp
  (bind _returnvalue (Transformation|GetActorTransform))
  (if (not (Utilities|IsValid (Variables|Default|GetPickUpActor)))
    (switch int (Math|Random|RandomIntegerinRange 0 3)
      (:0
        (bind _returnvalue_2 (Game|SpawnActorfromClass "/Game/Blueprints/BP_PickUp_ProjectileTiny.BP_PickUp_ProjectileTiny_C" (Math|Transform|MakeTransform (.location _returnvalue) "0, 0, 0" "1.000000,1.000000,1.000000") "Undefined" "MultiplyWithRoot" 0 0))
        (Variables|Default|SetPickUpActor _returnvalue_2))
      (:1
        (bind _returnvalue_3 (Game|SpawnActorfromClass "/Game/Blueprints/BP_PickUp_ProjectileNormal.BP_PickUp_ProjectileNormal_C" (Math|Transform|MakeTransform (.location _returnvalue) "0, 0, 0" "1.000000,1.000000,1.000000") "Undefined" "MultiplyWithRoot" 0 0))
        (Variables|Default|SetPickUpActor _returnvalue_3))
      (:2
        (bind _returnvalue_4 (Game|SpawnActorfromClass "/Game/Blueprints/BP_PickUp_ProjectileBig.BP_PickUp_ProjectileBig_C" (Math|Transform|MakeTransform (.location _returnvalue) "0, 0, 0" "1.000000,1.000000,1.000000") "Undefined" "MultiplyWithRoot" 0 0))
        (Variables|Default|SetPickUpActor _returnvalue_4))
      (:3
        (bind _returnvalue_5 (Game|SpawnActorfromClass "/Game/Blueprints/BP_PickUp_ProjectileBigger.BP_PickUp_ProjectileBigger_C" (Math|Transform|MakeTransform (.location _returnvalue) "0, 0, 0" "1.000000,1.000000,1.000000") "Undefined" "MultiplyWithRoot" 0 0))
        (Variables|Default|SetPickUpActor _returnvalue_5)))))