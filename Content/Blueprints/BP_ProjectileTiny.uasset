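; BP_ProjectileTiny is a small projectile that applies Chaos destruction when it hits a Geometry Collection actor.
; If the target simulates physics and has a primitive component, it wakes that body and adds an impulse built from only the projectile's X velocity.
; It also spawns a scaled-down FS_MasterField_Temp slightly behind the impact surface and triggers it as a short-lived radial field.
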(event OnComponentHit(CollisionComp)
  (params (HitComponent :type Primitive%20Component%20Object%20Reference) (OtherActor :type Actor%20Object%20Reference) (OtherComp :type Primitive%20Component%20Object%20Reference) (NormalImpulse :type Vector :default "0, 0, 0") (Hit :type Hit%20Result%20Structure%20%28by%20ref%29))
  (bind _returnvalue (Actor|GetComponentbyClass OtherActor "/Script/Engine.PrimitiveComponent"))
  (bind (_bblockinghit _binitialoverlap _time _distance _location _impactpoint _normal _impactnormal) (Collision|BreakHitResult Hit))
  (bind _returnvalue_2 (Math|Conversions|ToTransform(Vector) _impactpoint))
  (Utilities|Casting|CastToGeometryCollectionActor OtherActor)
  (if (Physics|IsSimulatingPhysics (Variables|/Script/Engine.Actor|GetRootComponent OtherActor) "None")
    (if (Utilities|IsValid _returnvalue)
      (Class|PrimitiveComponent|WakeRigidBody _returnvalue "None")
      (Physics|AddImpulseatLocation _returnvalue (Math|Conversions|ToVector(Float) (.X (Math|Vector|BreakVector (Transformation|GetVelocity)))) (Transformation|GetActorLocation) "None")))
  (bind _returnvalue_3 (Game|SpawnActorfromClass "/Game/Chaos/FS_MasterField_Temp.FS_MasterField_Temp_C" (Math|Transform|MakeTransform (+ (.location _returnvalue_2) (* _impactnormal "-3.000000,-3.000000,-3.000000")) (.rotation _returnvalue_2) "0.700000,0.700000,0.700000") "Undefined" "MultiplyWithRoot" 0 0))
  (Variables|Default|SetChaosImpactFieldReference _returnvalue_3)
  (Variables|/Game/Chaos/FS_MasterField_Temp.FS_MasterField_Temp_C|SetActivationType (Variables|Default|GetChaosImpactFieldReference) "NewEnumerator4")
  (Variables|/Game/Chaos/FS_MasterField_Temp.FS_MasterField_Temp_C|SetFieldLifespan (Variables|Default|GetChaosImpactFieldReference) 0.1)
  (Variables|/Game/Chaos/FS_MasterField_Temp.FS_MasterField_Temp_C|SetRadial%20Magnitude (Variables|Default|GetChaosImpactFieldReference) 1.5e+02)
  (Default|CETrigger (Variables|Default|GetChaosImpactFieldReference)))

(fn ConstructionScript)