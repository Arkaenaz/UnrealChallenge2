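; Projectile actor that pushes physics objects and sets off a Chaos field on impact.
; On collision hit, it applies an impulse at its own location to simulating targets, built only from the X component of its velocity.
; Every hit also spawns a scaled-down FS_MasterField_Temp just behind the impact surface, configures it as a short-lived radial field and triggers it immediately.
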(event OnComponentHit(CollisionComp)
  (params (HitComponent :type Primitive%20Component%20Object%20Reference) (OtherActor :type Actor%20Object%20Reference) (OtherComp :type Primitive%20Component%20Object%20Reference) (NormalImpulse :type Vector :default "0, 0, 0") (Hit :type Hit%20Result%20Structure%20%28by%20ref%29))
  (bind (_bblockinghit _binitialoverlap _time _distance _location _impactpoint _normal _impactnormal) (Collision|BreakHitResult Hit))
  (bind _returnvalue (Math|Conversions|ToTransform(Vector) _impactpoint))
  (if (Physics|IsSimulatingPhysics (Variables|/Script/Engine.Actor|GetRootComponent OtherActor) "None")
    (Physics|AddImpulseatLocation (Actor|GetComponentbyClass OtherActor "/Script/Engine.PrimitiveComponent") (Math|Conversions|ToVector(Float) (.X (Math|Vector|BreakVector (Transformation|GetVelocity)))) (Transformation|GetActorLocation) "None"))
  (bind _returnvalue_2 (Game|SpawnActorfromClass "/Game/Chaos/FS_MasterField_Temp.FS_MasterField_Temp_C" (Math|Transform|MakeTransform (+ (.location _returnvalue) (* _impactnormal "-3.000000,-3.000000,-3.000000")) (.rotation _returnvalue) "0.700000,0.700000,0.700000") "Undefined" "MultiplyWithRoot" 0 0))
  (Variables|Default|SetChaosImpactFieldReference _returnvalue_2)
  (Variables|/Game/Chaos/FS_MasterField_Temp.FS_MasterField_Temp_C|SetActivationType (Variables|Default|GetChaosImpactFieldReference) "NewEnumerator4")
  (Variables|/Game/Chaos/FS_MasterField_Temp.FS_MasterField_Temp_C|SetFieldLifespan (Variables|Default|GetChaosImpactFieldReference) 0.1)
  (Variables|/Game/Chaos/FS_MasterField_Temp.FS_MasterField_Temp_C|SetRadial%20Magnitude (Variables|Default|GetChaosImpactFieldReference) 1.5e+02)
  (Default|CETrigger (Variables|Default|GetChaosImpactFieldReference)))

(fn ConstructionScript)